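; Enemy turret that tracks the player and fires bullets at a fixed interval.
; Every tick it yaws its base toward the player pawn, leaving pitch and roll at zero.
; A looping timer started on BeginPlay plays a shot sound and spawns an enemy bullet at the Scene component's transform.
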(event `self.ReceiveBeginPlay`
  (`parent.ReceiveBeginPlay`)
  (`KismetSystemLibrary.K2_SetTimerDelegate` (delegate `ShootBullet`) 2.0 true))

(event `ShootBullet`
  (bind (_returnvalue_location _returnvalue_rotation) (`KismetMathLibrary.BreakTransform` (`SceneComponent.K2_GetComponentToWorld` (`self.Scene`))))
  (`GameplayStatics.PlaySound2D` "/Game/Sci-Fi_Shots_Pack2_Game_Of_Weapons/Wave/SciFi_Shot_P2__109_.SciFi_Shot_P2__109_" 0.25 1.0 0.0 null null)
  (`|SpawnActorFromClass` "/Game/Blueprints/BP_EnemyBullet.BP_EnemyBullet_C" (`KismetMathLibrary.MakeTransform` _returnvalue_location _returnvalue_rotation) "Undefined" "MultiplyWithRoot" null null))

(event `self.ReceiveTick`
  (params (DeltaSeconds :type "Float (single-precision)"))
  (bind (_returnvalue_roll _returnvalue_pitch _returnvalue_yaw) (`KismetMathLibrary.BreakRotator` (`KismetMathLibrary.FindLookAtRotation` (`self.K2_GetActorLocation`) (`self.K2_GetActorLocation` (`GameplayStatics.GetPlayerPawn` 0)))))
  (`SceneComponent.K2_SetWorldRotation` (`self.TurretBase`) (`KismetMathLibrary.MakeRotator` 0.0 0.0 _returnvalue_yaw) false false))

(fn `UserConstructionScript`
  (`parent.UserConstructionScript`))
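; Base enemy actor that takes damage, shows a health bar, and damages overlapping actors by its MaxHealth.
; AnyDamage reduces Health and updates the widget bar, then briefly flashes an overlay material on all static meshes if the enemy survives.
; Death plays sound and camera shake, reports score (MaxHealth) and a kill to the player controller, then spawns an explosion.
; An optional pickup, assigned through AssignSpawnedEnemyProps, also spawns before the actor is destroyed.
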(event `self.ReceiveAnyDamage`
  (params (Damage :type "Float (single-precision)") (DamageType :type "DamageType Object Reference") (InstigatedBy :type "Controller Object Reference") (DamageCauser :type "Actor Object Reference"))
  ; Projectile Damage
  (`self.ApplyDamage` Damage)
  ; Check if enemy health is 0, and if so start death
  (if (<= (`self.Health`) 0.0)
    ; Audio
    (`GameplayStatics.PlaySound2D` "/Game/Sci-Fi_Shots_Pack2_Game_Of_Weapons/Wave/SciFi_Shot_P2__40_.SciFi_Shot_P2__40_" 0.8 1.0 0.0 null null)
    ; Camera Shake
    (`|ExecutionSequence`
      (:`then_0`
        (bind _asmy_player_controller (cast `/Game/Framework/myPlayerController` (`GameplayStatics.GetPlayerController` 0)))
        (`/Game/Framework/myPlayerController.ApplyCameraShake` _asmy_player_controller)
        (message `/Game/Framework/BPI_myflyingshmup.SetPlayerScore` (`GameplayStatics.GetPlayerController` 0) (`self.Max Health`)))
      (:`then_1`
        ; Death Explosion
        (`|SpawnActorFromClass` "/Game/Particles/BP_Enemy_Death_Explosion.BP_Enemy_Death_Explosion_C" (`KismetMathLibrary.MakeTransform` (`self.K2_GetActorLocation`)) "AlwaysSpawn" "MultiplyWithRoot" null null)
        ; Pickup Spawn on death
        (if (`self.SpawnPickupOnDeath?`)
          (`|SpawnActorFromClass` (`self.PickupTypeToSpawn`) (`self.GetTransform`) "AlwaysSpawn" "MultiplyWithRoot" null null)))
      (:`then_2`
        (`self.K2_DestroyActor`))
      (:`then_3`
        (message `/Game/Framework/BPI_myflyingshmup.SetPlayerKillCount` (`GameplayStatics.GetPlayerController` 0) (`self.Kill`)))
      (:`then_4`
        (message `/Game/Framework/BPI_myflyingshmup.AddedScore` (`GameplayStatics.GetPlayerController` 0) (`self.Max Health`))))
    (else
      (`GameplayStatics.PlaySound2D` "/Game/Sci-Fi_Shots_Pack2_Game_Of_Weapons/Cue/SciFi_Shot_P2__158__Cue.SciFi_Shot_P2__158__Cue" 0.5 1.0 0.0 null null)
      ; Overlay Damage Flash
      (for _array_element (`self.K2_GetComponentsByClass` "/Script/Engine.StaticMeshComponent")
        (`MeshComponent.SetOverlayMaterial` _array_element "/Game/Materials/Mi_DamageFlash.Mi_DamageFlash"))
      (`KismetSystemLibrary.Delay` 0.2)
      (for _array_element_2 (`self.K2_GetComponentsByClass` "/Script/Engine.StaticMeshComponent")
        (`MeshComponent.SetOverlayMaterial` _array_element_2 null)))))

(event `self.ReceiveActorBeginOverlap`
  (params (OtherActor :type "Actor Object Reference"))
  ; Collison Damage
  (`GameplayStatics.ApplyDamage` OtherActor (`self.Max Health`)))

(event `self.ReceiveBeginPlay`
  ; Sets Health
  (set `self.Health` (`self.Max Health`)))

(event `ApplyDamage`
  (params (Damage :type "Float (double-precision)"))
  ; Applies and Reduces Damages
  (set `self.Health` (- (`self.Health`) Damage))
  ; Enemy Health bar Progress
  (bind _aswbp_enemy_health_bar (cast `/Game/Ui/WBP_EnemyHealthBar` (`WidgetComponent.GetUserWidgetObject` (`self.Widget`))))
  (`/Game/Ui/WBP_EnemyHealthBar.SetHealth` _aswbp_enemy_health_bar (/ (`self.Health`) (`self.Max Health`))))

(event `/Game/Framework/BPI_myflyingshmup.AssignSpawnedEnemyProps`
  (params (`SpawnPickupOnDeath?` :type Boolean) (PickupTypeToSpawn :type "/Game/Blueprints/PickUpBps/BP_BasePickup Class Reference"))
  (set `self.SpawnPickupOnDeath?` `SpawnPickupOnDeath?`)
  (set `self.PickupTypeToSpawn` PickupTypeToSpawn))

(fn `UserConstructionScript`)
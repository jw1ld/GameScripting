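; Boss enemy that slides into the play area along X on a timeline, then moves side to side along Y with a second timeline.
; Tick yaws both turret bases toward the player, using the look-at angle from the boss's center.
; A looping timer calls Shoot, whose parallel Delay branches stagger bullet fire from a front transform array, two turret points and two rear points, so the delays set each weapon's cadence.
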(event `EnterPlayArea`
  ; Boss Movement
  (set `self.InitalLocation` (`self.K2_GetActorLocation`))
  (bind (_direction _x_offset) (`Timeline|Timeline` :!via `PlayFromStart`)
    (:`Update`
      (`self.K2_SetActorLocation` (+ (`self.InitalLocation`) (`KismetMathLibrary.MakeVector` (* _x_offset -2000.0))) true))
    (:`Finished`
      (`self.MoveSideToSide`))))

(event `MoveSideToSide`
  ; Boss Movement
  (set `self.InitalLocation` (`self.K2_GetActorLocation`))
  (`TimelineComponent.SetPlayRate` (`self.Timeline_0`) 0.05)
  (bind (_direction _y_value) (`Timeline|Timeline_0` :!via `PlayFromStart`)
    (:`Update`
      (`self.K2_SetActorLocation` (+ (`self.InitalLocation`) (`KismetMathLibrary.MakeVector` 0.0 (* _y_value 3000.0))) true))))

(event `self.ReceiveBeginPlay`
  (`parent.ReceiveBeginPlay`)
  (`self.EnterPlayArea`)
  (`KismetSystemLibrary.K2_SetTimerDelegate` (delegate `Shoot`) 1.0 true true))

(event `Shoot`
  (bind (_returnvalue_location _returnvalue_rotation) (`KismetMathLibrary.BreakTransform` (`SceneComponent.K2_GetComponentToWorld` (`self.Scene`))))
  (bind (_returnvalue_location_2 _returnvalue_rotation_2) (`KismetMathLibrary.BreakTransform` (`SceneComponent.K2_GetComponentToWorld` (`self.ShootingPoint2`))))
  (bind (_returnvalue_location_3 _returnvalue_rotation_3 _returnvalue_scale) (`KismetMathLibrary.BreakTransform` (`SceneComponent.K2_GetComponentToWorld` (`self.Arrow`))))
  (bind (_returnvalue_location_4 _returnvalue_rotation_4) (`KismetMathLibrary.BreakTransform` (`SceneComponent.K2_GetComponentToWorld` (`self.ShootingPoint1`))))
  (bind (_returnvalue_location_5 _returnvalue_rotation_5) (`KismetMathLibrary.BreakTransform` (`SceneComponent.K2_GetComponentToWorld` (`self.Scene2`))))
  (`|ExecutionSequence`
    (:`then_0`
      ; Front Shooting
      (`KismetSystemLibrary.Delay` 6.0)
      (`GameplayStatics.PlaySound2D` "/Game/Sci-Fi_Shots_Pack2_Game_Of_Weapons/Wave/SciFi_Shot_P2__109_.SciFi_Shot_P2__109_" 0.25 1.0 0.0 null null)
      (for _array_element (`self.ShootingTransforms`)
        (`|SpawnActorFromClass` "/Game/Blueprints/BP_EnemyBullet.BP_EnemyBullet_C" (`KismetMathLibrary.MakeTransform` (+ (.location _array_element) _returnvalue_location_3) (`KismetMathLibrary.ComposeRotators` (.rotation _array_element) _returnvalue_rotation_3) (+ _returnvalue_scale (.scale _array_element))) "Undefined" "MultiplyWithRoot" null null)))
    (:`then_1`
      ; Turret shooting
      (`KismetSystemLibrary.Delay` 2.0)
      (`GameplayStatics.PlaySound2D` "/Game/Sci-Fi_Shots_Pack2_Game_Of_Weapons/Wave/SciFi_Shot_P2__109_.SciFi_Shot_P2__109_" 0.25 1.0 0.0 null null)
      (`|SpawnActorFromClass` "/Game/Blueprints/BP_EnemyBullet.BP_EnemyBullet_C" (`KismetMathLibrary.MakeTransform` _returnvalue_location _returnvalue_rotation) "Undefined" "MultiplyWithRoot" null null))
    (:`then_2`
      (`KismetSystemLibrary.Delay` 2.0)
      (`GameplayStatics.PlaySound2D` "/Game/Sci-Fi_Shots_Pack2_Game_Of_Weapons/Wave/SciFi_Shot_P2__109_.SciFi_Shot_P2__109_" 0.25 1.0 0.0 null null)
      (`|SpawnActorFromClass` "/Game/Blueprints/BP_EnemyBullet.BP_EnemyBullet_C" (`KismetMathLibrary.MakeTransform` _returnvalue_location_5 _returnvalue_rotation_5) "Undefined" "MultiplyWithRoot" null null))
    (:`then_3`
      ; Rear Shooting
      (`KismetSystemLibrary.Delay` 4.0)
      (`GameplayStatics.PlaySound2D` "/Game/Sci-Fi_Shots_Pack2_Game_Of_Weapons/Wave/SciFi_Shot_P2__109_.SciFi_Shot_P2__109_" 0.25 1.0 0.0 null null)
      (`|SpawnActorFromClass` "/Game/Blueprints/BP_EnemyBullet.BP_EnemyBullet_C" (`KismetMathLibrary.MakeTransform` _returnvalue_location_4 _returnvalue_rotation_4) "Undefined" "MultiplyWithRoot" null null))
    (:`then_4`
      (`KismetSystemLibrary.Delay` 4.0)
      (`GameplayStatics.PlaySound2D` null 1.0 1.0 0.0 null null)
      (`|SpawnActorFromClass` "/Game/Blueprints/BP_EnemyBullet.BP_EnemyBullet_C" (`KismetMathLibrary.MakeTransform` _returnvalue_location_2 _returnvalue_rotation_2) "Undefined" "MultiplyWithRoot" null null))))

(event `self.ReceiveTick`
  (params (DeltaSeconds :type "Float (single-precision)"))
  (bind (_returnvalue_roll _returnvalue_pitch _returnvalue_yaw) (`KismetMathLibrary.BreakRotator` (`KismetMathLibrary.FindLookAtRotation` (`self.K2_GetActorLocation`) (`self.K2_GetActorLocation` (`GameplayStatics.GetPlayerPawn` 0)))))
  ; Tracking
  (`SceneComponent.K2_SetWorldRotation` (`self.TurretBase`) (`KismetMathLibrary.MakeRotator` 0.0 0.0 _returnvalue_yaw) false false)
  (`SceneComponent.K2_SetWorldRotation` (`self.TurretBase2`) (`KismetMathLibrary.MakeRotator` 0.0 0.0 _returnvalue_yaw) false false))

(fn `UserConstructionScript`
  (`parent.UserConstructionScript`))
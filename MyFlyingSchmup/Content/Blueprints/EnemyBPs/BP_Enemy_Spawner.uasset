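; Enemy spawner that repeatedly spawns a random enemy class from a pool at random intervals of a few seconds.
; A timer event spawns each enemy at a random point on a start spline, facing a random point on an end spline, then re-queues itself.
; Each enemy receives a randomly chosen pickup type and a weighted chance to drop it on death.
; All randomness comes from one fixed-seed random stream.
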(event `self.ReceiveBeginPlay`
  (`KismetMathLibrary.SetRandomStreamSeed` (`self.RandomStream`) 32434)
  (`self.queueEnemysPAWN`))

(event `queueEnemysPAWN`
  (bind _returnvalue (`KismetSystemLibrary.K2_SetTimerDelegate` (delegate `Spawn Enemy`) (`KismetMathLibrary.RandomFloatInRangeFromStream` (`self.RandomStream`) 1.0 5.0) false true))
  (set `self.Enemy Spawn Timer` _returnvalue))

(event `Spawn Enemy`
  (bind (_startlocation_ _end_location) (`self.GetStartandEndlocation`))
  (bind _returnvalue (`|SpawnActorFromClass` (`KismetArrayLibrary.Array_RandomFromStream` (`self.Enemy Class Pool`) (`self.RandomStream`)) (`KismetMathLibrary.MakeTransform` _startlocation_ (`KismetMathLibrary.FindLookAtRotation` _startlocation_ _end_location)) "Undefined" "MultiplyWithRoot" null null))
  (message `/Game/Framework/BPI_myflyingshmup.AssignSpawnedEnemyProps` _returnvalue (`KismetMathLibrary.RandomBoolWithWeightFromStream` (`self.RandomStream`)) (`KismetArrayLibrary.Array_RandomFromStream` (`self.PickupClassPool`) (`self.RandomStream`)))
  (`self.queueEnemysPAWN`))

(event `self.ReceiveActorBeginOverlap`
  (params (OtherActor :type "Actor Object Reference")))

(fn `GetStartandEndlocation`
  (returns (`StartLocation'` :type "Vector Structure") (`End Location` :type "Vector Structure"))
  (bind _returnvalue (`KismetMathLibrary.RandomFloatFromStream` (`self.RandomStream`)))
  (return (`SplineComponent.GetLocationAtTime` (`self.StartLoc`) _returnvalue "World" false) (`SplineComponent.GetLocationAtTime` (`self.EndLoc`) _returnvalue "World" false)))

(fn `UserConstructionScript`)
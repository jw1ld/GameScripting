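; BP_Enemy_A is an enemy actor that automatically and repeatedly fires bullets during play.
; On BeginPlay, a looping timer calls Shoot, which plays a 2D sci-fi shot sound and spawns BP_EnemyBullet at the BulletSpawnPoint transform.
; Shoot repeats the sound and spawn after a Delay equal to the timer interval, so follow-up shots coincide with later timer ticks.
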(event `self.ReceiveBeginPlay`
  (`KismetSystemLibrary.K2_SetTimerDelegate` (delegate `Shoot`) 1.0 true true))

(event `Shoot`
  (`GameplayStatics.PlaySound2D` "/Game/Sci-Fi_Shots_Pack2_Game_Of_Weapons/Wave/SciFi_Shot_P2__109_.SciFi_Shot_P2__109_" 0.25 1.0 0.0 null null)
  (`|SpawnActorFromClass` "/Game/Blueprints/BP_EnemyBullet.BP_EnemyBullet_C" (`SceneComponent.K2_GetComponentToWorld` (`self.BulletSpawnPoint`)) "Undefined" "MultiplyWithRoot" null null)
  (`KismetSystemLibrary.Delay` 1.0)
  (`GameplayStatics.PlaySound2D` "/Game/Sci-Fi_Shots_Pack2_Game_Of_Weapons/Wave/SciFi_Shot_P2__109_.SciFi_Shot_P2__109_" 0.25 1.0 0.0 null null)
  (`|SpawnActorFromClass` "/Game/Blueprints/BP_EnemyBullet.BP_EnemyBullet_C" (`SceneComponent.K2_GetComponentToWorld` (`self.BulletSpawnPoint`)) "Undefined" "MultiplyWithRoot" null null))

(fn `UserConstructionScript`)
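; BP_EnemyOnPath is an enemy Blueprint that travels along its own spline path.
; On BeginPlay it detaches the spline, keeping its world transform, so the path stays put as the actor moves.
; A timeline with play rate scaled by the inverse of TravelTime samples the spline by time and moves the actor there with sweep, leaving rotation untouched.
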(event `self.ReceiveBeginPlay`
  (`parent.ReceiveBeginPlay`)
  (`SceneComponent.K2_DetachFromComponent` (`self.Spline`) "KeepWorld" "KeepWorld" "KeepWorld" true)
  (`TimelineComponent.SetPlayRate` (`self.MoveAlongSpline`) (/ 1.0 (`self.Travel Time`)))
  (bind (_direction _time) (`Timeline|MoveAlongSpline` :!via `PlayFromStart`)
    (:`Update`
      (`self.K2_SetActorLocation` (`SplineComponent.GetLocationAtTime` (`self.Spline`) _time "World" false) true))))

(fn `UserConstructionScript`
  (`parent.UserConstructionScript`))
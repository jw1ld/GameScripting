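; BP_Enemy_C is an enemy that automatically fires bullet patterns on a looping timer started at BeginPlay.
; Each shot plays a 2D sound, then spawns one BP_EnemyBullet for every entry in the ShootingTransform array.
; Each entry offsets the BulletSpawnPoint world transform: location and scale are added, so location offsets ignore the spawn point's rotation, while rotations are combined.
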(event `self.ReceiveBeginPlay`
  (`KismetSystemLibrary.K2_SetTimerDelegate` (delegate `Shoot`) 1.5 true true))

(event `Shoot`
  (bind (_returnvalue_location _returnvalue_rotation _returnvalue_scale) (`KismetMathLibrary.BreakTransform` (`SceneComponent.K2_GetComponentToWorld` (`self.BulletSpawnPoint`))))
  (`GameplayStatics.PlaySound2D` "/Game/Sci-Fi_Shots_Pack2_Game_Of_Weapons/Wave/SciFi_Shot_P2__109_.SciFi_Shot_P2__109_" 0.25 1.0 0.0 null null)
  (for _array_element (`self.ShootingTransform`)
    (`|SpawnActorFromClass` "/Game/Blueprints/BP_EnemyBullet.BP_EnemyBullet_C" (`KismetMathLibrary.MakeTransform` (+ (.location _array_element) _returnvalue_location) (`KismetMathLibrary.ComposeRotators` (.rotation _array_element) _returnvalue_rotation) (+ _returnvalue_scale (.scale _array_element))) "Undefined" "MultiplyWithRoot" null null)))

(fn `UserConstructionScript`)